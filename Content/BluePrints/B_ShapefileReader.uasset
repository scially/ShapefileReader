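; B_ShapefileReader is an actor that demonstrates the ShapefileReader plugin by loading its bundled School.shp and printing its contents on BeginPlay.
; It builds the file path from the project directory and stores the loaded reader if valid.
; It then fetches features by index, using the reader's FieldCount as the loop bound, and prints each valid feature's "xqmc" field and center X coordinate.
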(event EventBeginPlay
  (bind _returnvalue (Class|ShapefileReaderLibrary|ReadShapefile (Class|BlueprintPathsLibrary|Combine (Utilities|Array|MakeArray (Utilities|Paths|GetPath (Class|BlueprintPathsLibrary|GetProjectFilePath)) "Plugins\\ShapefileReader\\Resources\\Data\\School.shp"))))
  (if (Utilities|IsValid _returnvalue)
    (Variables|Default|SetShapefileReader _returnvalue)
    (for _index (range 0 (- (Variables|/Script/ShapefileReader.ShapefileReaderRecord|GetFieldCount (Variables|Default|GetShapefileReader)) 1))
      (if (Utilities|IsValid (Class|ShapefileReaderRecord|GetShapefileFeature (Variables|Default|GetShapefileReader) _index))
        (Variables|Default|SetShapefileFeature (Class|ShapefileReaderRecord|GetShapefileFeature (Variables|Default|GetShapefileReader) _index))
        (Development|PrintString (Class|ShapefileFeature|GetFieldasString (Variables|Default|GetShapefileFeature) "xqmc") true true "(R=0.000000,G=0.660000,B=1.000000,A=1.000000)" 8.0)
        (Development|PrintString (Utilities|String|ToString(Float) (.x (Variables|/Script/ShapefileReader.ShapefileFeature|GetCenter (Variables|Default|GetShapefileFeature)))))))))

(fn ConstructionScript)